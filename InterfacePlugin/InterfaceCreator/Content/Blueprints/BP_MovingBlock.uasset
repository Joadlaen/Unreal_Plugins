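; Interactable block actor that moves and rotates once when interacted with, using a mesh assigned through the construction script.
; OnInteract checks CanInteract and NotMoved, then plays the BoxMove timeline, which clears NotMoved when finished.
; Each update lerps location and rotation toward per-axis offsets from the current transform rather than a cached start, so movement accumulates and the final displacement differs from the set offsets.
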(event `/Game/Interfaces/BPI_Interact.OnInteract`
  (params (CanInteract :type Boolean))
  (bind (_returnvalue_x _returnvalue_y _returnvalue_z) (`KismetMathLibrary.BreakVector` (`self.K2_GetActorLocation`)))
  (bind (_returnvalue_roll _returnvalue_pitch _returnvalue_yaw) (`KismetMathLibrary.BreakRotator` (`self.K2_GetActorRotation`)))
  (if CanInteract
    (if (`self.NotMoved`)
      (`TimelineComponent.SetPlayRate` (`self.BoxMove`) 1.0)
      (bind (_direction _boxmove1) (`Timeline|BoxMove`)
        (:`Update`
          (`self.K2_SetActorLocationAndRotation` (`KismetMathLibrary.MakeVector` (`KismetMathLibrary.Lerp` _returnvalue_x (+ _returnvalue_x (`self.NewX`)) _boxmove1) (`KismetMathLibrary.Lerp` _returnvalue_y (+ _returnvalue_y (`self.NewY`)) _boxmove1) (`KismetMathLibrary.Lerp` _returnvalue_z (+ _returnvalue_z (`self.NewZ`)) _boxmove1)) (`KismetMathLibrary.MakeRotator` (`KismetMathLibrary.Lerp` _returnvalue_roll (+ _returnvalue_roll (`self.NewRoll`)) _boxmove1) (`KismetMathLibrary.Lerp` _returnvalue_pitch (+ _returnvalue_pitch (`self.NewPitch`)) _boxmove1) (`KismetMathLibrary.Lerp` _returnvalue_yaw (+ _returnvalue_yaw (`self.NewYaw`)) _boxmove1))))
        (:`Finished`
          (set `self.NotMoved` false))))))

(fn `UserConstructionScript`
  (`StaticMeshComponent.SetStaticMesh` (`self.StaticMesh`) (`self.New Mesh`)))